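; Road spawner that builds a chain of Road_bp segments in the level, laying an initial run on BeginPlay.
; The first segment spawns at a hard-coded location, and each following one at the newest road's RoadSpawnPoint, clearing StartOfRoad.
; Each spawned segment becomes NewestRoad and receives a reference back to the spawner in its RoadSpawn variable.
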(event EventBeginPlay
  (CallFunction|InitalRoadStart))

(fn ConstructionScript)

(fn RoadSpawner
  (params (Spawn%20Road%20Location :type Vector))
  (bind _returnvalue (Game|SpawnActorfromClass "/Game/Blueprints/Road_bp.Road_bp_C" (Math|Transform|MakeTransform Spawn%20Road%20Location "0, 0, 0" "1,1,1") "Undefined" 0 0))
  (bind _output_get (Variables|Default|SetNewest_Road _returnvalue))
  (Variables|/Game/Blueprints/Road_bp.Road_bp_C|SetRoad_spawn _output_get self))

(fn SpawnRoadatSpawnpoint
  (CallFunction|RoadSpawner (Transformation|GetWorldLocation (Variables|/Game/Blueprints/Road_bp.Road_bp_C|GetRoad_spawn_point (Variables|Default|GetNewest_Road)))))

(fn InitalRoadStart
  (for _index (range 0 3)
    (Utilities|IsValid (Variables|Default|GetNewest_Road)
      (:Is%20Valid
        (Variables|Default|SetStart%20of%20Road false)
        (CallFunction|SpawnRoadatSpawnpoint))
      (:Is%20Not%20Valid
        (CallFunction|RoadSpawner "-550.000000,1060.000000,120.000000")))))