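; TrainLight_BP is a train light Blueprint that flashes a left and a right light alternately.
; Tick runs through a 0.2-second Delay, which throttles the toggle to roughly that interval.
; Each toggle reads the left light's intensity to pick which light goes to full brightness and which goes dark, so no separate state variable is used.
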(event EventBeginPlay)

(event Collision|EventActorBeginOverlap
  (params (OtherActor :type Actor%20Object%20Reference)))

(event EventTick
  (params (DeltaSeconds :type Float%20%28single-precision%29))
  (Utilities|FlowControl|Delay 0.2)
  (if (== (Variables|/Script/Engine.LightComponentBase|GetIntensity (Variables|Default|Getleft%20Light)) 5e+03)
    (Rendering|Components|Light|SetIntensity (Variables|Default|Getleft%20Light) 0.0)
    (Rendering|Components|Light|SetIntensity (Variables|Default|Getright%20Light) 5e+03)
    (else
      (Rendering|Components|Light|SetIntensity (Variables|Default|Getleft%20Light) 5e+03)
      (Rendering|Components|Light|SetIntensity (Variables|Default|Getright%20Light) 0.0))))

(fn ConstructionScript)