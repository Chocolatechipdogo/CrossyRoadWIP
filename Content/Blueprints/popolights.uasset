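; Blueprint with red and blue light components that re-orient repeatedly, apparently as flashing police lights.
; Tick passes through a 0.2-second Delay, throttling the calls to the two events that update each light.
; Each event keeps the light's location and derives a new rotation by treating its roll, pitch and negated yaw as an X-axis direction vector.
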(event Custom|add%20red%20light
  (bind _red_light (Variables|Default|GetRed%20Light))
  (bind _returnvalue (Transformation|GetWorldRotation _red_light))
  (Transformation|SetWorldLocationAndRotation _red_light (Transformation|GetWorldLocation _red_light) (Math|Conversions|RotationFromXVector (Math|Vector|MakeVector (.roll _returnvalue) (.pitch _returnvalue) (* (.yaw _returnvalue) -1.0))) false false))

(event Custom|add%20blue%20light
  (bind _blue_light (Variables|Default|GetBlue%20Light))
  (bind _returnvalue (Transformation|GetWorldRotation _blue_light))
  (Transformation|SetWorldLocationAndRotation _blue_light (Transformation|GetWorldLocation _blue_light) (Math|Conversions|RotationFromXVector (Math|Vector|MakeVector (.roll _returnvalue) (.pitch _returnvalue) (* (.yaw _returnvalue) -1.0))) false false))

(event EventTick
  (params (DeltaSeconds :type Float%20%28single-precision%29))
  (Utilities|FlowControl|Delay 0.2)
  (CallFunction|AddRedLight)
  (CallFunction|AddBlueLight))

(fn ConstructionScript)