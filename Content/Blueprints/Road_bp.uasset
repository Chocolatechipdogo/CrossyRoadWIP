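; Lane actor for a Crossy Road-style chicken game that randomly becomes grass with trees, car road, railroad or river on BeginPlay.
; It spawns one car, log or train with warning light, moves it each Tick in a random direction, and end triggers respawn it after random delays.
; Player overlap requests the next lane from RoadSpawn and, on exit, destroys this one after a delay; rivers kill the player.
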(event OnComponentBeginOverlap(Road_Trigger)
  (params (OverlappedComponent :type Primitive%20Component%20Object%20Reference) (OtherActor :type Actor%20Object%20Reference) (OtherComp :type Primitive%20Component%20Object%20Reference) (OtherBodyIndex :type Integer) (bFromSweep :type Boolean) (SweepResult :type Hit%20Result%20Structure%20%28by%20ref%29))
  ;[1 1 1] Spawn More road
  (Utilities|Casting|CastToThirdPersonCharacter OtherActor)
  (Default|SpawnRoadatSpawnpoint (Variables|Default|GetRoad_spawn)))

(event OnComponentBeginOverlap(RiverCollision)
  (params (OverlappedComponent :type Primitive%20Component%20Object%20Reference) (OtherActor :type Actor%20Object%20Reference) (OtherComp :type Primitive%20Component%20Object%20Reference) (OtherBodyIndex :type Integer) (bFromSweep :type Boolean) (SweepResult :type Hit%20Result%20Structure%20%28by%20ref%29))
  ;[1 1 1] Drowning chicken code
  (bind _asthird_person_character (Utilities|Casting|CastToThirdPersonCharacter OtherActor))
  (if (Variables|Default|Getriver?)
    (Default|ChickenGotHit _asthird_person_character)
    (Transformation|SetWorldScale3D (Variables|/Game/ThirdPersonBP/Blueprints/ThirdPersonCharacter.ThirdPersonCharacter_C|GetChicken _asthird_person_character) "0.001000,0.001000,0.001000")))

(event OnComponentEndOverlap(Road_Trigger)
  (params (OverlappedComponent :type Primitive%20Component%20Object%20Reference) (OtherActor :type Actor%20Object%20Reference) (OtherComp :type Primitive%20Component%20Object%20Reference) (OtherBodyIndex :type Integer))
  (bind _the_log (Variables|Default|GetThe_Log))
  (bind _the_train (Variables|Default|GetThe%20Train))
  (bind _the_car (Variables|Default|Getthe_car))
  ;[1 1 1] Destroy lanes
  (bind _asthird_person_character (Utilities|Casting|CastToThirdPersonCharacter OtherActor))
  (if (not (Variables|/Game/ThirdPersonBP/Blueprints/ThirdPersonCharacter.ThirdPersonCharacter_C|GetDEAD _asthird_person_character))
    (Utilities|FlowControl|Delay 1e+01)
    (Actor|DestroyActor)
    (Utilities|IsValid _the_car
      (:Is%20Valid
        (Default|SelfDistruct _the_car))
      (:Is%20Not%20Valid
        (Utilities|IsValid _the_log
          (:Is%20Valid
            (Default|SelfDistruct _the_log))
          (:Is%20Not%20Valid
            (Utilities|IsValid _the_train
              (:Is%20Valid
                (Default|SelfDestruct _the_train)
                (Default|SelfDestruct (Variables|Default|GetTheLight))))))))))

(event OnComponentBeginOverlap(Trigger_begin)
  (params (OverlappedComponent :type Primitive%20Component%20Object%20Reference) (OtherActor :type Actor%20Object%20Reference) (OtherComp :type Primitive%20Component%20Object%20Reference) (OtherBodyIndex :type Integer) (bFromSweep :type Boolean) (SweepResult :type Hit%20Result%20Structure%20%28by%20ref%29))
  (bind _returnvalue (Math|Random|RandomFloatinRange 5.0 1e+01))
  ;[1 1 1] respawning of moving objects
  (if (not (Variables|Default|GetSafe%20Zone))
    (if (Variables|Default|Getriver?)
      (bind _aslog_bp (Utilities|Casting|CastToLog_BP OtherActor))
      (if (not (== (Variables|Default|GetLeft%20or%20right) 0))
        (Default|SelfDistruct _aslog_bp)
        (Utilities|FlowControl|Delay (Math|Random|RandomFloatinRange 0.5 3.0))
        (CallFunction|SpawnLog (Variables|Default|GetLeft%20or%20right)))
      (elif (Variables|Default|Gettrain?)
        (bind _astrain_bp (Utilities|Casting|CastToTRAIN_bp OtherActor))
        (if (not (== (Variables|Default|GetLeft%20or%20right) 0))
          (Default|SelfDestruct _astrain_bp)
          (if (> _returnvalue 5.0)
            (for _index (range 0 (Math|Float|Truncate (- _returnvalue 5.0)))
              (CallFunction|WarningLights)
              (Utilities|FlowControl|Delay 5.0)
              (CallFunction|TurnWarningOff)
              (CallFunction|SpawnTrain (Variables|Default|GetLeft%20or%20right)))
            (Utilities|FlowControl|Delay 5.0)
            (CallFunction|TurnWarningOff)
            (else
              (CallFunction|WarningLights)
              (Utilities|FlowControl|Delay _returnvalue)
              (CallFunction|TurnWarningOff)))
          (CallFunction|SpawnTrain (Variables|Default|GetLeft%20or%20right)))
        (else
          (bind _ascar_bp (Utilities|Casting|CastToCar_bp OtherActor))
          (if (not (== (Variables|Default|GetLeft%20or%20right) 0))
            (Default|SelfDistruct _ascar_bp)
            (Utilities|FlowControl|Delay (Math|Random|RandomFloatinRange 2.0 5.0))
            (CallFunction|SpawnCar (Variables|Default|GetLeft%20or%20right))))))))

(event OnComponentBeginOverlap(Trigger_beginR)
  (params (OverlappedComponent :type Primitive%20Component%20Object%20Reference) (OtherActor :type Actor%20Object%20Reference) (OtherComp :type Primitive%20Component%20Object%20Reference) (OtherBodyIndex :type Integer) (bFromSweep :type Boolean) (SweepResult :type Hit%20Result%20Structure%20%28by%20ref%29))
  (bind _returnvalue (Math|Random|RandomFloatinRange 5.0 1e+01))
  ;[1 1 1] respawning of moving objects
  (if (not (Variables|Default|GetSafe%20Zone))
    (if (Variables|Default|Getriver?)
      (bind _aslog_bp (Utilities|Casting|CastToLog_BP OtherActor))
      (if (not (== (Variables|Default|GetLeft%20or%20right) 1))
        (Default|SelfDistruct _aslog_bp)
        (Utilities|FlowControl|Delay (Math|Random|RandomFloatinRange 0.5 3.0))
        (CallFunction|SpawnLog (Variables|Default|GetLeft%20or%20right)))
      (elif (Variables|Default|Gettrain?)
        (bind _astrain_bp (Utilities|Casting|CastToTRAIN_bp OtherActor))
        (if (not (== (Variables|Default|GetLeft%20or%20right) 1))
          (Default|SelfDestruct _astrain_bp)
          (if (> _returnvalue 5.0)
            (for _index (range 0 (Math|Float|Truncate (- _returnvalue 5.0)))
              (CallFunction|WarningLights)
              (Utilities|FlowControl|Delay 5.0)
              (CallFunction|TurnWarningOff)
              (CallFunction|SpawnTrain (Variables|Default|GetLeft%20or%20right)))
            (Utilities|FlowControl|Delay 5.0)
            (CallFunction|TurnWarningOff)
            (else
              (CallFunction|WarningLights)
              (Utilities|FlowControl|Delay _returnvalue)
              (CallFunction|TurnWarningOff)))
          (CallFunction|SpawnTrain (Variables|Default|GetLeft%20or%20right)))
        (else
          (bind _ascar_bp (Utilities|Casting|CastToCar_bp OtherActor))
          (if (not (== (Variables|Default|GetLeft%20or%20right) 1))
            (Default|SelfDistruct _ascar_bp)
            (Utilities|FlowControl|Delay (Math|Random|RandomFloatinRange 1.0 5.0))
            (CallFunction|SpawnCar (Variables|Default|GetLeft%20or%20right))))))))

(event Custom|Warning%20lights
  (bind _thelight (Variables|Default|GetTheLight))
  (bind _left_light (Variables|/Game/Blueprints/TrainLight_BP.TrainLight_BP_C|Getleft%20Light _thelight))
  ;[1 1 1] Light Warning Switching
  (Utilities|IsValid _thelight
    (:Is%20Valid
      (Utilities|FlowControl|Delay 0.2)
      (if (== (Variables|/Script/Engine.LightComponentBase|GetIntensity _left_light) 0.0)
        (Rendering|Components|Light|SetIntensity _left_light 7e+03)
        (else
          (Rendering|Components|Light|SetIntensity _left_light 0.0)
          (Rendering|Components|Light|SetIntensity (Variables|/Game/Blueprints/TrainLight_BP.TrainLight_BP_C|Getright%20Light _thelight) 7e+03))))))

(event Custom|Turn%20Warning%20Off
  (bind _thelight (Variables|Default|GetTheLight))
  ;[1 1 1] Turn off WarningLights
  (Utilities|IsValid _thelight
    (:Is%20Valid
      (Rendering|Components|Light|SetIntensity (Variables|/Game/Blueprints/TrainLight_BP.TrainLight_BP_C|Getleft%20Light _thelight) 0.0)
      (Rendering|Components|Light|SetIntensity (Variables|/Game/Blueprints/TrainLight_BP.TrainLight_BP_C|Getright%20Light _thelight) 0.0))))

(event EventBeginPlay
  ;[1 1 1] Sets type of lane and what should should spawn
  (bind _asthird_person_character (Utilities|Casting|CastToThirdPersonCharacter (Game|GetPlayerCharacter 0)))
  (Variables|Default|SetThe%20Chicken _asthird_person_character)
  (Variables|Default|SetLeftEndOfTheRoad (Transformation|GetWorldLocation (Variables|Default|GetSpawn_start)))
  (Variables|Default|SetRightEndOfTheRoad (Transformation|GetWorldLocation (Variables|Default|GetSpawn_startR)))
  (bind _output_get (Variables|Default|SetLeft%20or%20right (Math|Random|RandomIntegerinRange 0 1)))
  (if (== _output_get 1)
    (Variables|Default|SetMoving%20vehicle (* (Variables|Default|GetMoving%20vehicle) -1.0))
    (Variables|Default|SetTrain%20Speed (* (Variables|Default|GetTrain%20Speed) -1.0)))
  (CallFunction|RandomLanes (Math|Random|RandomIntegerinRange 0 8))
  (if (Variables|Default|GetSafe%20Zone)
    (Game|SpawnActorfromClass "/Game/Blueprints/Tree_bp.Tree_bp_C" (Math|Transform|MakeTransform (Math|Vector|MakeVector (.x (Variables|Default|GetLeftEndOfTheRoad)) (.y (Variables|Default|GetLeftEndOfTheRoad)) (- (.z (Variables|Default|GetLeftEndOfTheRoad)) 1e+02)) "0, 0, 0" "1,1,1") "Undefined" 0 0)
    (Game|SpawnActorfromClass "/Game/Blueprints/Tree_bp.Tree_bp_C" (Math|Transform|MakeTransform (Math|Vector|MakeVector (.x (Variables|Default|GetRightEndOfTheRoad)) (.y (Variables|Default|GetRightEndOfTheRoad)) (- (.z (Variables|Default|GetRightEndOfTheRoad)) 1e+02)) "0, 0, 0" "1,1,1") "Undefined" 0 0)
    (switch int (Math|Random|RandomIntegerinRange 0 1)
      (:1
        ;[1 1 1] Spawn Trees on Grass
        (for _index (range 0 (Math|Float|Truncate (/ (Math|Vector|Distance(Vector) (Variables|Default|GetLeftEndOfTheRoad) (Variables|Default|GetRightEndOfTheRoad)) 6e+01)))
          (if (> (Math|Random|RandomFloat) 0.8)
            (Game|SpawnActorfromClass "/Game/Blueprints/Tree_bp.Tree_bp_C" (Math|Transform|MakeTransform (Math|Vector|MakeVector (+ (Math|Conversions|ToFloat(Integer) (* _index 90)) (.X (Math|Vector|BreakVector (Variables|Default|GetLeftEndOfTheRoad)))) (.y (Variables|Default|GetLeftEndOfTheRoad)) (- (.z (Variables|Default|GetLeftEndOfTheRoad)) 1e+02)) "0, 0, 0" "1,1,1") "Undefined" 0 0)))))
    (elif (Variables|Default|Getriver?)
      (CallFunction|SpawnLog (Variables|Default|GetLeft%20or%20right))
      (elif (Variables|Default|Gettrain?)
        (CallFunction|SpawnTrainLight)
        (CallFunction|SpawnTrain (Variables|Default|GetLeft%20or%20right))
        (else
          (CallFunction|SpawnCar (Variables|Default|GetLeft%20or%20right)))))))

(event EventTick
  (params (DeltaSeconds :type Float%20%28single-precision%29))
  (bind _the_train (Variables|Default|GetThe%20Train))
  (bind _the_log (Variables|Default|GetThe_Log))
  (bind _the_car (Variables|Default|Getthe_car))
  (bind _moving_vehicle (Variables|Default|GetMoving%20vehicle))
  (bind _returnvalue (* DeltaSeconds _moving_vehicle))
  ;[1 1 1] Vechiel Movement
  (Utilities|FlowControl|Sequence
    (:then_0
      (Utilities|IsValid _the_car
        (:Is%20Valid
          (Transformation|AddActorWorldOffset _the_car (Math|Vector|MakeVector _returnvalue 0.0 0.0) true))
        (:Is%20Not%20Valid
          (Utilities|IsValid _the_log
            (:Is%20Valid
              (Transformation|AddActorWorldOffset _the_log (Math|Vector|MakeVector _returnvalue 0.0 0.0) true))
            (:Is%20Not%20Valid
              (Utilities|IsValid _the_train
                (:Is%20Valid
                  (Transformation|AddActorWorldOffset _the_train (Math|Vector|MakeVector (* DeltaSeconds (Variables|Default|GetTrain%20Speed)) 0.0 0.0) true))))))))))

(fn ConstructionScript)

(fn RandomLanes
  (params (Select%20Lane :type Integer))
  (Variables|Default|SetSafe%20Zone (Math|Boolean|ORBoolean (== Select%20Lane 0) (== Select%20Lane 1) (== Select%20Lane 6) (== Select%20Lane 7) (== Select%20Lane 8)))
  (Variables|Default|Setriver? (== Select%20Lane 5))
  (Variables|Default|Settrain? (== Select%20Lane 4))
  (Components|StaticMesh|SetStaticMesh (Variables|Default|GetRoad) (Utilities|Select :Index Select%20Lane :Option%200 "/Game/Meshes/untitled.untitled" :Option%201 "/Game/Meshes/grass_2_0.grass_2_0" :Option%202 "/Game/Meshes/beginRoad.beginRoad" :Option%203 "/Game/Meshes/DAROAD.DAROAD" :Option%204 "/Game/Meshes/Railroad.Railroad" :Option%205 "/Game/Meshes/River.River" :Option%206 "/Game/Meshes/untitled.untitled" :Option%207 "/Game/Meshes/grass_2_0.grass_2_0" :Option%208 "/Game/Meshes/untitled.untitled")))

(fn CarSpawn
  (params (Car%20spawn%20START :type Vector) (Spawn%20Transform%20Rotation :type Rotator))
  (bind _returnvalue (Game|SpawnActorfromClass "/Game/Blueprints/Car_bp.Car_bp_C" (Math|Transform|MakeTransform Car%20spawn%20START Spawn%20Transform%20Rotation "1,1,1") "Undefined" 0 0))
  (Variables|Default|Setthe_car _returnvalue))

(fn SpawnCar
  (params (Left%20or%20right :type Integer))
  (bind _spawn_start (Variables|Default|GetSpawn_start))
  (bind _spawn_startr (Variables|Default|GetSpawn_startR))
  (bind _returnvalue (Utilities|Select :Index Left%20or%20right :Option%200 _spawn_start :Option%201 _spawn_startr))
  (bind _returnvalue_2 (Transformation|GetWorldLocation _returnvalue))
  (if (== Left%20or%20right 1)
    (bind _output_get (Variables|Default|Setrotation%20of%20vechiel "-180.000000, 0, 0"))
    (CallFunction|CarSpawn _returnvalue_2 (Math|Conversions|RotationFromXVector _output_get))
    (else
      (bind _output_get_2 (Variables|Default|Setrotation%20of%20vechiel "0, 0, 0"))
      (CallFunction|CarSpawn _returnvalue_2 (Math|Conversions|RotationFromXVector _output_get_2)))))

(fn LogSpawner
  (params (Spawn%20Transform%20Location :type Vector) (Spawn%20Transform%20Rotation :type Rotator))
  (bind _returnvalue (Game|SpawnActorfromClass "/Game/Blueprints/Log_BP.Log_BP_C" (Math|Transform|MakeTransform Spawn%20Transform%20Location Spawn%20Transform%20Rotation "1,1,1") "Undefined" 0 0))
  (Variables|Default|SetThe_Log _returnvalue))

(fn SpawnLog
  (params (Left%20or%20Right? :type Integer))
  (bind _spawn_start (Variables|Default|GetSpawn_start))
  (bind _spawn_startr (Variables|Default|GetSpawn_startR))
  (bind _returnvalue (Utilities|Select :Index Left%20or%20Right? :Option%200 _spawn_start :Option%201 _spawn_startr))
  (bind _returnvalue_2 (Transformation|GetWorldLocation _returnvalue))
  (bind _returnvalue_3 (* _returnvalue_2 "1.000000,1.000000,0.500000"))
  (if (== Left%20or%20Right? 1)
    (bind _output_get (Variables|Default|Setrotation%20of%20vechiel "-180.000000, 0, 0"))
    (CallFunction|LogSpawner _returnvalue_3 (Math|Conversions|RotationFromXVector _output_get))
    (else
      (bind _output_get_2 (Variables|Default|Setrotation%20of%20vechiel "0, 0, 0"))
      (CallFunction|LogSpawner _returnvalue_3 (Math|Conversions|RotationFromXVector _output_get_2)))))

(fn TrainSpawner
  (params (Spawn%20Transform%20Rotation :type Rotator) (Spawn%20Transform%20Location :type Vector))
  (bind _returnvalue (Game|SpawnActorfromClass "/Game/Blueprints/TRAIN_bp.TRAIN_bp_C" (Math|Transform|MakeTransform Spawn%20Transform%20Location Spawn%20Transform%20Rotation "1,1,1") "Undefined" 0 0))
  (Variables|Default|SetThe%20Train _returnvalue))

(fn SpawnTrain
  (params (Left%20or%20Right :type Integer))
  (bind _spawn_start (Variables|Default|GetSpawn_start))
  (bind _spawn_startr (Variables|Default|GetSpawn_startR))
  (bind _returnvalue (Utilities|Select :Index 0 :Option%200 _spawn_start :Option%201 _spawn_startr))
  (bind _returnvalue_2 (Transformation|GetWorldLocation _returnvalue))
  (if (== Left%20or%20Right 1)
    (bind _output_get (Variables|Default|Setrotation%20of%20vechiel "-180.000000, 0, 0"))
    (CallFunction|TrainSpawner (Math|Conversions|RotationFromXVector _output_get) _returnvalue_2)
    (else
      (bind _output_get_2 (Variables|Default|Setrotation%20of%20vechiel "0, 0, 0"))
      (CallFunction|TrainSpawner (Math|Conversions|RotationFromXVector _output_get_2) _returnvalue_2))))

(fn TrainLightSpawner
  (params (Light%20Location :type Vector))
  (bind _returnvalue (Game|SpawnActorfromClass "/Game/Blueprints/TrainLight_BP.TrainLight_BP_C" (Math|Transform|MakeTransform Light%20Location "0, 0, 0" "1,1,1") "Undefined" 0 0))
  (Variables|Default|SetTheLight _returnvalue))

(fn SpawnTrainLight
  (CallFunction|TrainLightSpawner (Transformation|GetWorldLocation (Variables|Default|GettrainLight%20placement))))