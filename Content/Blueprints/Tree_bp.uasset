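; Placeable scenery actor that appears as either its default Tree mesh or a rock, and removes itself after the player character passes.
; On BeginPlay a coin-flip random either keeps the mesh or swaps it to Rock and lowers it slightly.
; When a ThirdPersonCharacter stops overlapping the Box, the actor waits a fixed delay and then destroys itself.
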(event OnComponentEndOverlap(Box)
  (params (OverlappedComponent :type Primitive%20Component%20Object%20Reference) (OtherActor :type Actor%20Object%20Reference) (OtherComp :type Primitive%20Component%20Object%20Reference) (OtherBodyIndex :type Integer))
  (Utilities|Casting|CastToThirdPersonCharacter OtherActor)
  (Utilities|FlowControl|Delay 1e+01)
  (Actor|DestroyActor))

(event EventBeginPlay
  (bind _tree (Variables|Default|GetTree))
  (bind _returnvalue (Transformation|GetWorldLocation _tree))
  (switch int (Math|Random|RandomIntegerinRange 0 1)
    (:1
      (Components|StaticMesh|SetStaticMesh (Variables|Default|GetTree) "/Game/Meshes/rock.rock")
      (Transformation|SetWorldLocation _tree (Math|Vector|MakeVector (.x _returnvalue) (.y _returnvalue) (- (.Z (Math|Vector|BreakVector (Transformation|GetWorldLocation _tree))) 3e+01)) false false))))

(fn ConstructionScript)