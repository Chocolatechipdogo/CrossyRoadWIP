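; Obstacle actor, either a vehicle or a log, that squashes the player's chicken character when it hits.
; On BeginPlay the Car flag picks a random bus or beetle mesh, or the log mesh when false.
; The first character to overlap the Box is flattened by scaling and notified through ChickenGotHit, guarded by a DoOnce.
; A SelfDistruct event destroys the actor after a short delay.
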(event OnComponentBeginOverlap(Box)
  (params (OverlappedComponent :type Primitive%20Component%20Object%20Reference) (OtherActor :type Actor%20Object%20Reference) (OtherComp :type Primitive%20Component%20Object%20Reference) (OtherBodyIndex :type Integer) (bFromSweep :type Boolean) (SweepResult :type Hit%20Result%20Structure%20%28by%20ref%29))
  (bind _asthird_person_character (Utilities|Casting|CastToThirdPersonCharacter OtherActor))
  (Utilities|FlowControl|DoOnce false
    (:Completed
      (Transformation|SetWorldScale3D (Variables|/Script/Engine.Actor|GetRootComponent _asthird_person_character) "0.500000,0.500000,0.100000")
      (Default|ChickenGotHit _asthird_person_character))))

(event Custom|Self%20Distruct
  (Utilities|FlowControl|Delay 0.5)
  (Actor|DestroyActor))

(event EventBeginPlay
  (CallFunction|RandomCar (Variables|Default|GetCar?)))

(event EventTick
  (params (DeltaSeconds :type Float%20%28single-precision%29)))

(fn ConstructionScript)

(fn RandomCar
  (params (car? :type Boolean))
  (bind _bus (Variables|Default|GetBus))
  (if car?
    (Components|StaticMesh|SetStaticMesh _bus (Utilities|Select :Index (Math|Random|RandomIntegerinRange 0 1) :Option%200 "/Game/Meshes/Cars/Bus.Bus" :Option%201 "/Game/Meshes/Cars/Beetle_Car.Beetle_Car" :Option%202 0))
    (else
      (Components|StaticMesh|SetStaticMesh _bus "/Game/Meshes/Cars/log.log"))))

(fn Log)